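; BP_Robot1 is a player-controlled robot shooter that moves on world X/Y axes and turns its mesh toward the mouse cursor.
; While not Muerto, Tick sets mesh yaw toward a point projected along the cursor ray; the accompanying line trace's result is unused.
; Holding left mouse sets Disparando on BP_animacion and spawns BP_BALA from both pistols, rate-limited by a timer resetting Bala.
; InterseccionPlanorecta is empty and Disparar ignores its Offset.
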(event `self.ReceiveTick`
  (params (DeltaSeconds :type "Float (single-precision)"))
  (bind _returnvalue (`GameplayStatics.GetPlayerController` 0))
  (bind _mesh (`self.Mesh`))
  (bind (_locationx _locationy) (`PlayerController.GetMousePosition` _returnvalue))
  (bind (_worldposition _worlddirection) (`GameplayStatics.DeprojectScreenToWorld` _returnvalue (`KismetMathLibrary.MakeVector2D` _locationx _locationy)))
  (bind _returnvalue_2 (+ _worldposition (* _worlddirection 1000)))
  (if (not (`self.Muerto`))
    (`KismetSystemLibrary.LineTraceSingle` _worldposition _returnvalue_2 "TraceTypeQuery1")
    (`SceneComponent.K2_SetWorldRotation` _mesh (`KismetMathLibrary.MakeRotator` 0.0 0.0 (- (.yaw (`KismetMathLibrary.FindLookAtRotation` (.location (`SceneComponent.K2_GetComponentToWorld` _mesh)) _returnvalue_2)) 90.0)) false false)
    (if (`self.Disparo`)
      (if (`self.bala`)
        (`self.Disparar` 0.25)
        (set `self.bala` false)
        (`KismetSystemLibrary.K2_SetTimer` null "Puede Disparar?" 0.2)))))

(event `InputAxis|MovimientoAdelante`
  (params (AxisValue :type "Float (single-precision)"))
  (`self.AddMovementInput` (1.0 0.0 0.0) AxisValue))

(event `InputAxis|MovimientoDerecha`
  (params (AxisValue :type "Float (single-precision)"))
  (`self.AddMovementInput` (0.0 1.0 0.0) AxisValue))

(event `Key|LeftMouseButton`
  (params (Key :type "Key Structure"))
  (bind _disparo (`self.Disparo`))
  (bind _returnvalue (`SkeletalMeshComponent.GetAnimInstance` (`self.Mesh`)))
  (:`Pressed`
    (set `self.Disparo` true)
    (bind _asbp_animacion (cast `/Game/Personajes/BP_animacion` _returnvalue))
    (set `/Game/Personajes/BP_animacion.Disparando` _disparo _asbp_animacion))
  (:`Released`
    (set `self.Disparo` false)
    (bind _asbp_animacion_2 (cast `/Game/Personajes/BP_animacion` _returnvalue))
    (set `/Game/Personajes/BP_animacion.Disparando` _disparo _asbp_animacion_2)))

(fn `Disparar`
  (params (Offset :type "Float (double-precision)"))
  (`|ExecutionSequence`
    (:`then_0`
      (set `self.Posicion` (`SceneComponent.K2_GetComponentToWorld` (`self.Pistola1`))))
    (:`then_1`
      (set `self.Posicion` (`SceneComponent.K2_GetComponentToWorld` (`self.Pistola2`)))))
  (`|SpawnActorFromClass` "/Game/Particulas/BP_BALA.BP_BALA_C" (`self.Posicion`) "Undefined" "OverrideRootScale" null null))

(fn `Interseccion plano/recta`)

(fn `Puede Disparar?`
  (set `self.bala` true))

(fn `UserConstructionScript`)