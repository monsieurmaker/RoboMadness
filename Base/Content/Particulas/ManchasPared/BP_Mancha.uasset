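; BP_Mancha is a short-lived stain decal actor with a randomized look, mostly blood splatters and smears.
; The construction script uses a random MultiGate to set the decal material from blood variants and one yellow paint splatter, with some smear materials repeated across outputs.
; Tick accumulates elapsed time in Contador and destroys the actor after five seconds.
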(event `self.ReceiveBeginPlay`)

(event `self.ReceiveTick`
  (params (DeltaSeconds :type "Float (single-precision)"))
  (bind _output_get (set `self.contador` (+ DeltaSeconds (`self.contador`))))
  (if (>= _output_get 5.0)
    (`self.K2_DestroyActor`)))

(fn `UserConstructionScript`
  (bind _decal (`self.Decal`))
  (`|MultiGate` true
    (:`Out 0`
      (`DecalComponent.SetDecalMaterial` _decal "/Game/TextureMax/SplatterDecals/M_Blood_Master.M_Blood_Master"))
    (:`Out 1`
      (`DecalComponent.SetDecalMaterial` _decal "/Game/TextureMax/SplatterDecals/Materials/M_Blood_Smear_01b_Inst.M_Blood_Smear_01b_Inst"))
    (:`Out 2`
      (`DecalComponent.SetDecalMaterial` _decal "/Game/Particulas/ManchasPared/Materials/M_Blood_Smear_01c_Inst.M_Blood_Smear_01c_Inst"))
    (:`Out 3`
      (`DecalComponent.SetDecalMaterial` _decal "/Game/Particulas/ManchasPared/Materials/M_Blood_Smear_01c_Inst.M_Blood_Smear_01c_Inst"))
    (:`Out 4`
      (`DecalComponent.SetDecalMaterial` _decal "/Game/Particulas/ManchasPared/Materials/M_Blood_Smear_01b_Inst.M_Blood_Smear_01b_Inst"))
    (:`Out 5`
      (`DecalComponent.SetDecalMaterial` _decal "/Game/TextureMax/SplatterDecals/Materials/M_Blood_Smear_01d_Inst.M_Blood_Smear_01d_Inst"))
    (:`Out 6`
      (`DecalComponent.SetDecalMaterial` _decal "/Game/TextureMax/SplatterDecals/Materials/M_Paint_Yellow_Splatter_04.M_Paint_Yellow_Splatter_04"))
    (:`Out 7`
      (`DecalComponent.SetDecalMaterial` _decal "/Game/TextureMax/SplatterDecals/Materials/M_Blood_Smear_01d_Inst.M_Blood_Smear_01d_Inst"))))