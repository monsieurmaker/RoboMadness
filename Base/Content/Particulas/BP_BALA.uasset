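; BP_BALA is a bullet actor that leaves splat decals where it hits and hurts BP_gris targets.
; Its construction script uses a random MultiGate to pick a blue, red or green mesh material.
; On hit it spawns a BP_Mancha aligned to the surface normal with randomized decal roll and size, then destroys itself.
; BP_gris hits also call Pupa, adding an impulse along the normal once Vida drops below zero.
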(event `self.ReceiveHit`
  (params (MyComp :type "PrimitiveComponent Object Reference") (Other :type "Actor Object Reference") (OtherComp :type "PrimitiveComponent Object Reference") (bSelfMoved :type Boolean) (HitLocation :type "Vector Structure") (HitNormal :type "Vector Structure") (NormalImpulse :type "Vector Structure") (Hit :type "HitResult Structure (by ref)"))
  (`/Engine/EditorBlueprintResources/StandardMacros.IsValid` Other
    (:`Is Valid`
      (`/Engine/EditorBlueprintResources/StandardMacros.IsValid` OtherComp
        (:`Is Valid`
          (if (not (== Other self))
            (bind _returnvalue (`|SpawnActorFromClass` "/Game/Particulas/ManchasPared/BP_Mancha.BP_Mancha_C" (`KismetMathLibrary.MakeTransform` HitLocation (`KismetMathLibrary.MakeRotFromZ` HitNormal)) "Undefined" "OverrideRootScale" null null))
            (bind _decal (`DecalActor.Decal` _returnvalue))
            (`SceneComponent.K2_AddLocalRotation` _decal (`KismetMathLibrary.MakeRotator` (`KismetMathLibrary.RandomFloatInRange` 0.0 360.0)) false false)
            (`SceneComponent.SetWorldScale3D` _decal (`KismetMathLibrary.MakeVector` (`KismetMathLibrary.RandomFloatInRange` 0.1 0.6) 0.15 (`KismetMathLibrary.RandomFloatInRange` 0.1 0.6)))
            (if (== (`GameplayStatics.GetObjectClass` Other) "/Game/Enemigos/BP_gris.BP_gris_C")
              (bind _asbp_gris (cast `/Game/Enemigos/BP_gris` Other))
              (`/Game/Enemigos/BP_gris.pupa` _asbp_gris)
              (if (< (`/Game/Enemigos/BP_gris.Vida` _asbp_gris) 0.0)
                (`PrimitiveComponent.AddImpulseAtLocation` OtherComp HitNormal HitLocation "None")
                (`KismetSystemLibrary.PrintText` "Hello")))
            (`self.K2_DestroyActor` :!label _label)))
        (:`Is Not Valid`
          (goto _label))))
    (:`Is Not Valid`
      (goto _label))))

(fn `UserConstructionScript`
  (bind _staticmeshcomponent (`self.StaticMeshComponent`))
  (`|MultiGate` true
    (:`Out 0`
      (`PrimitiveComponent.SetMaterial` _staticmeshcomponent 0 "/Game/Particulas/Azul.Azul"))
    (:`Out 1`
      (`PrimitiveComponent.SetMaterial` _staticmeshcomponent 0 "/Game/Particulas/Rojo.Rojo"))
    (:`Out 2`
      (`PrimitiveComponent.SetMaterial` _staticmeshcomponent 0 "/Game/Particulas/Verde.Verde"))))