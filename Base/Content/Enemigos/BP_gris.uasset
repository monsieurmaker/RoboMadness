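; BP_gris is an enemy actor with health (Vida) that blinks and is then destroyed when that health drops below zero.
; The pupa event subtracts a fixed amount of health, and Tick checks for the death condition.
; A self-restarting timeline toggles skeletal mesh visibility, while the Borrar timeline delays DestroyActor.
; The sphere overlap only prints a debug greeting for BP_Robot1.
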(event `self.ReceiveTick`
  (params (DeltaSeconds :type "Float (single-precision)"))
  (if (< (`self.Vida`) 0.0)
    (`Timeline|Línea de tiempo_0` :!label _label
      (:`Finished`
        (`|ExecutionSequence`
          (:`then_0`
            (bind _output_get (set `self.visible` (not (`self.visible`))))
            (`SceneComponent.SetVisibility` (`self.SkeletalMesh`) _output_get false)
            (goto _label :!via `PlayFromStart`))
          (:`then_1`
            (`Timeline|Borrar`
              (:`Finished`
                (`self.K2_DestroyActor`)))))))))

(event `self.Sphere.OnComponentBeginOverlap`
  (params (OverlappedComponent :type "PrimitiveComponent Object Reference") (OtherActor :type "Actor Object Reference") (OtherComp :type "PrimitiveComponent Object Reference") (OtherBodyIndex :type Integer) (bFromSweep :type Boolean) (SweepResult :type "HitResult Structure (by ref)"))
  (if (== OtherActor "/Game/Personajes/BP_Robot1.BP_Robot1")
    (`KismetSystemLibrary.PrintText` "Hello")))

(event `pupa`
  (set `self.Vida` (- (`self.Vida`) 3.0)))

(fn `toggleVisibility`
  (`SceneComponent.SetVisibility` (`self.SkeletalMesh`) false false))

(fn `UserConstructionScript`)